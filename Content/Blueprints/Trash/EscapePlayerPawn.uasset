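; EscapePlayerPawn is a player pawn with a camera that follows controller rotation and a toggle crouch.
; Each tick it sets the camera height from BaseEyeHeight, rotates ControlHip and Camera to the controller's desired rotation, and turns the actor by yaw only.
; Crouch input alternates through a FlipFlop that sets IsCrouched and plays or reverses a timeline, interpolating BaseEyeHeight between standing and crouched values.
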(event `self.ReceiveBeginPlay`)

(event `self.ReceiveTick`
  (params (DeltaSeconds :type "Float (single-precision)"))
  (bind _returnvalue (`Controller.GetDesiredRotation` (`self.GetController`)))
  (`SceneComponent.K2_SetRelativeLocation` (`self.Camera`) (`KismetMathLibrary.MakeVector` 0.0 0.0 (`self.BaseEyeHeight`)) false false)
  (`SceneComponent.K2_SetWorldRotation` (`self.ControlHip`) _returnvalue false false)
  (`SceneComponent.K2_SetWorldRotation` (`self.Camera`) _returnvalue false false)
  (`self.K2_SetActorRotation` (`KismetMathLibrary.MakeRotator` 0.0 0.0 (.yaw _returnvalue))))

(event `InputAction|Crouch`
  (params (Key :type "Key Structure"))
  (:`Pressed`
    (`/Engine/EditorBlueprintResources/StandardMacros.FlipFlop`
      (:`A`
        (set `self.IsCrouched` true)
        (bind (_direction _newtrack_0) (`Timeline|Timeline_0` :!label _label)
          (:`Update`
            (set `self.BaseEyeHeight` (`KismetMathLibrary.Lerp` 80.0 30.0 _newtrack_0)))))
      (:`B`
        (set `self.IsCrouched` false)
        (goto _label :!via `Reverse`)))))

(fn `UserConstructionScript`)
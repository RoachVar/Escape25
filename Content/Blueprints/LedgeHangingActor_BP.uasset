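; Helper actor for ledge hanging that moves and rotates the actor it is attached to into a hang position.
; Straight adjustments use a timeline blend, with location also smoothed by constant-speed interpolation.
; Corner adjustments chain two timelines through a midpoint computed in the start rotation's local space.
; Both snap to the target and call AdjustmentEnded on finish; a SetParameters call for overriding defaults is left unconnected.
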(event `self.ReceiveBeginPlay`)

(event `self.AdjustLocationToHangPosition`
  (params (HangLocation :type "Vector Structure") (HangRotation :type "Rotator Structure"))
  (bind _returnvalue (`self.GetAttachParentActor`))
  (bind _returnvalue_2 (`self.GetAttachParentActor`))
  ;[1 1 1] Blending tp hang location
  (set `self.BlendEndLocation` HangLocation)
  (set `self.BlendEndRotation` HangRotation)
  (set `self.BlendStartRotation` (`self.K2_GetActorRotation`))
  (set `self.BlendStartLocation` (`self.K2_GetActorLocation`))
  (bind (_direction _blend) (`Timeline|AdjustmentToHangPositionBlend` :!via `PlayFromStart`)
    (:`Update`
      (`self.K2_SetActorLocation` _returnvalue (`KismetMathLibrary.VInterpTo_Constant` (`self.K2_GetActorLocation`) (`KismetMathLibrary.VLerp` (`self.BlendStartLocation`) (`self.BlendEndLocation`) _blend) (`GameplayStatics.GetWorldDeltaSeconds`) 700.0) false true)
      (`self.K2_SetActorRotation` _returnvalue (`KismetMathLibrary.RLerp` (`self.BlendStartRotation`) (`self.BlendEndRotation`) _blend true) true))
    (:`Finished`
      (`self.K2_SetActorLocation` _returnvalue_2 (`self.BlendEndLocation`) false true)
      (`self.K2_SetActorRotation` _returnvalue_2 (`self.BlendEndRotation`) true)
      (`self.AdjustmentEnded`))))

(event `self.AdjustLocationAroundCorner`
  (params (HangLocation :type "Vector Structure") (HangRotation :type "Rotator Structure"))
  (bind _returnvalue (`self.GetAttachParentActor`))
  (bind _returnvalue_2 (`self.GetAttachParentActor`))
  (bind _returnvalue_3 (`self.GetAttachParentActor`))
  ;[1 1 1] Blending around corner
  (set `self.BlendEndLocation` HangLocation)
  (set `self.BlendEndRotation` HangRotation)
  (set `self.BlendStartRotation` (`self.K2_GetActorRotation`))
  (set `self.BlendStartLocation` (`self.K2_GetActorLocation`))
  (set `self.BlendMidPoint` (+ (`self.BlendStartLocation`) (`KismetMathLibrary.GreaterGreater_VectorRotator` (`KismetMathLibrary.MakeVector` 0.0 (.y (`KismetMathLibrary.LessLess_VectorRotator` (- (`self.BlendEndLocation`) (`self.BlendStartLocation`)) (`self.BlendStartRotation`))) (.z (`KismetMathLibrary.LessLess_VectorRotator` (- (`self.BlendEndLocation`) (`self.BlendStartLocation`)) (`self.BlendStartRotation`)))) (`self.K2_GetActorRotation`))))
  (set `self.BlendMidRotation` (`KismetMathLibrary.ComposeRotators` (`self.BlendStartRotation`) (* (`self.BlendEndRotation`) 0.5)))
  (bind (_direction _blend) (`Timeline|BlendToCornerMidPoint` :!via `PlayFromStart`)
    (:`Update`
      (`self.K2_SetActorLocation` _returnvalue_3 (`KismetMathLibrary.VInterpTo_Constant` (`self.K2_GetActorLocation`) (`KismetMathLibrary.VLerp` (`self.BlendStartLocation`) (`self.BlendMidPoint`) _blend) (`GameplayStatics.GetWorldDeltaSeconds`) 700.0) false true)
      (`self.K2_SetActorRotation` _returnvalue_3 (`KismetMathLibrary.RLerp` (`self.BlendStartRotation`) (`self.BlendMidRotation`) 0.0 true) true))
    (:`Finished`
      (bind (_direction_2 _blend_2) (`Timeline|BlendFromMidpointToCorner` :!via `PlayFromStart`)
        (:`Update`
          (`self.K2_SetActorLocation` _returnvalue_2 (`KismetMathLibrary.VLerp` (`self.BlendMidPoint`) (`self.BlendEndLocation`) _blend_2) false true)
          (`self.K2_SetActorRotation` _returnvalue_2 (`KismetMathLibrary.RLerp` (`self.BlendMidRotation`) (`self.BlendEndRotation`) _blend_2 true) true))
        (:`Finished`
          (`self.K2_SetActorLocation` _returnvalue (`self.BlendEndLocation`) false true)
          (`self.K2_SetActorRotation` _returnvalue (`self.BlendEndRotation`) true)
          (`self.AdjustmentEnded`))))))

(fn `UserConstructionScript`)
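; Base interactable component that shows an on-screen indicator widget reflecting its focus state.
; On each focus state change it creates the indicator if the state is Marked and none exists, binding it to itself and the first player controller.
; It forwards every state change to a live indicator and clears its reference when the indicator reports its death, allowing a new one later.
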(event `self.ReceiveBeginPlay`
  (add `self.FocusStateChanged` (delegate `OnFocusStateChanged`)))

(event `OnFocusStateChanged`
  (bind _returnvalue (`self.GetFocusState`))
  (bind _ownedindicator (`self.OwnedIndicator`))
  (`|ExecutionSequence`
    (:`then_0`
      (switch `EFocusState` _returnvalue
        (:`MarkedState`
          (`self.AddIndicator`))))
    (:`then_1`
      (`/Engine/EditorBlueprintResources/StandardMacros.IsValid` _ownedindicator
        (:`Is Valid`
          (`/Game/Widgets/Indicator.StateChanged` _ownedindicator _returnvalue))))))

(event `AddIndicator`
  (`/Engine/EditorBlueprintResources/StandardMacros.IsValid` (`self.OwnedIndicator`)
    (:`Is Not Valid`
      (bind _returnvalue (`|CreateWidget` "/Game/Widgets/Indicator.Indicator_C" (`GameplayStatics.GetPlayerController` 0) (`self.Object Name`) self))
      (bind _output_get (set `self.OwnedIndicator` _returnvalue))
      (add `/Game/Widgets/Indicator.ReportDeath` _output_get (delegate `IndicatorExpired`))
      (`UserWidget.AddToViewport` (`self.OwnedIndicator`) 0))))

(event `IndicatorExpired`
  (set `self.OwnedIndicator` null))
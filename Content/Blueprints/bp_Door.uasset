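; Interactable door Blueprint that swings its mesh open and closed on yaw through a timeline.
; Interaction toggles the state through ChangeIfOpened, swaps the Open/Close display row from a data table and sets the interactable component inactive.
; Closing reverses the timeline, but when not player-triggered it first waits on an optional delay timer, which reopening cancels.
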(event `self.Interactable_Base.InteractionStart`
  (set `self.PlayerInteracted` true)
  (`self.ChangeIfOpened` (not (`self.IsOpened`)))
  (`ActorComponent.SetActive` (`self.Interactable_Base`) false false))

(event `ChangeIfOpened`
  (params (IsOpened :type Boolean))
  (bind _output_get (set `self.IsOpened` IsOpened))
  (set `/Game/Blueprints/Interactable_Base.InteractionDisplay` (make `DataTableRowHandle` "/Game/Data/dt_InteractionDisplayData.dt_InteractionDisplayData" (select `bool` _output_get :`false` "Open" :`true` "Close" :!type "Name")) (`self.Interactable_Base`))
  (`|ExecutionSequence`
    (:`then_0`
      (if (`self.IsOpened`)
        (`KismetSystemLibrary.K2_InvalidateTimerHandle` (`self.ClosingDelay`))
        (bind (_direction _blend) (`Timeline|DoorOpening` :!label _label)
          (:`Update`
            (`SceneComponent.K2_SetRelativeRotation` (`self.StaticMeshComponent0`) (`KismetMathLibrary.MakeRotator` 0.0 0.0 (`KismetMathLibrary.Lerp` 0.0 90.0 _blend)) false false)))
        (elif (and (> (`self.DelayBeforeClosing`) 0.0) (not (`self.PlayerInteracted`)))
          (`self.StartClosingDelay`)
          (else
            (goto _label :!via `Reverse`)))))
    (:`then_1`
      (set `self.PlayerInteracted` false))))

(event `ClosingDelayEnded`
  (goto _label :!via `Reverse`))

(event `StartClosingDelay`
  (bind _returnvalue (`KismetSystemLibrary.K2_SetTimerDelegate` (`|CreateDelegate` :!event `ClosingDelayEnded`) (`self.DelayBeforeClosing`)))
  (set `self.ClosingDelay` _returnvalue))

(fn `UserConstructionScript`)